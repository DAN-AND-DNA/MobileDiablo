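; Main menu player controller that lets the player hover and pick a hero.
; Each tick it clears the previous hover, finds the closest hero target under a small radius, and highlights it and the selected hero via custom depth stencil on mesh and equipment.
; The SelectHero input swaps the selection, fires the hero-selected callback and caches the hero ID in the map cache subsystem.
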(event Custom|HighlightHoverTarget
  ;[1 1 1] highlight hover target
  (bind _returnvalue (Class|MobileDiabloMainMenuPlayerController|GetClosestTarget false 2e+01))
  (bind _asbp_hero (Utilities|Casting|CastToBP_Hero _returnvalue))
  (bind _output_get (Variables|Default|SetHoveredHero _asbp_hero))
  (Utilities|IsValid _output_get
    (:Is%20Valid
      (Rendering|SetCustomDepthStencilValue (Variables|/Script/Engine.Character|GetMesh _output_get) 4)
      (Class|ShowEquipmentComponent|SetCustomDepthStencilValue (Variables|/Script/MobileDiablo.MobileDiabloCharacter|GetShowEquipmentComp _output_get) 4))))

(event Custom|CleanHighlightHoverTarget
  ;[1 1 1 1 20] clean highlight hover target
  (Utilities|IsValid (Variables|Default|GetHoveredHero)
    (:Is%20Valid
      (Rendering|SetCustomDepthStencilValue (Variables|/Script/Engine.Character|GetMesh (Variables|Default|GetHoveredHero)) 1)
      (Class|ShowEquipmentComponent|SetCustomDepthStencilValue (Variables|/Script/MobileDiablo.MobileDiabloCharacter|GetShowEquipmentComp (Variables|Default|GetHoveredHero)) 1)
      (Variables|Default|SetHoveredHero 0))))

(event EventTick
  (params (DeltaSeconds :type Float%20%28single-precision%29))
  (bind _selectedhero (Variables|Default|GetSelectedHero))
  (CallFunction|CleanHighlightHoverTarget)
  (CallFunction|HighlightHoverTarget)
  (Utilities|IsValid _selectedhero
    (:Is%20Valid
      (Rendering|SetCustomDepthStencilValue (Variables|/Script/Engine.Character|GetMesh _selectedhero) 4)
      (Class|ShowEquipmentComponent|SetCustomDepthStencilValue (Variables|/Script/MobileDiablo.MobileDiabloCharacter|GetShowEquipmentComp _selectedhero) 4))))

(event Input|ActionEvents|InputActionSelectHero
  (params (Key :type Key%20Structure :default "None"))
  (bind _hoveredhero (Variables|Default|GetHoveredHero))
  ;[1 1 1 1 20] Input
  (:Pressed
    (Utilities|IsValid (Variables|Default|GetSelectedHero)
      (:Is%20Valid
        (Rendering|SetCustomDepthStencilValue (Variables|/Script/Engine.Character|GetMesh (Variables|Default|GetSelectedHero)) 1)
        (Class|ShowEquipmentComponent|SetCustomDepthStencilValue (Variables|/Script/MobileDiablo.MobileDiabloCharacter|GetShowEquipmentComp (Variables|Default|GetSelectedHero)) 1)
        (Variables|Default|SetSelectedHero 0)
        (Default|CallOnHeroSelected))
      (:Is%20Not%20Valid
        _))
    (Utilities|IsValid _hoveredhero
      (:Is%20Valid
        (bind _output_get (Variables|Default|SetSelectedHero _hoveredhero))
        (Default|CallOnHeroSelected)
        (Class|MobileDiabloMapCacheSubsystem|SetValue (Subsystems|GetMobileDiabloMapCacheSubsystem) "Key_MainMenu_SelectedHeroID" (Utilities|String|ToString(Name) (Variables|/Script/MobileDiablo.MobileDiabloCharacter|GetHeroID _output_get)))
        (Development|PrintString (Utilities|String|ToString(Name) (Variables|/Script/MobileDiablo.MobileDiabloCharacter|GetHeroID _output_get)))))))

(fn ConstructionScript)